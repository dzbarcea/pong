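; Pong-style ball actor that bounces between paddles, tracks both sides' scores and ends the match.
; Overlaps drive physics velocity: paddles flip Y and set X from paddle velocity plus random spread, while horizontal boundaries flip X.
; Goals recenter and relaunch the ball, then update the score on tagged TextRender actors.
; When a score exceeds ten, it sets GameOver, and Tick stops the ball and reopens P1_Main after a delay.
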(event EventBeginPlay
  (Physics|SetPhysicsLinearVelocity (Variables|Default|GetStaticMesh) "0.000000,2000.000000, 0" false "None"))

(event Collision|EventActorBeginOverlap
  (params (OtherActor :type Actor%20Object%20Reference))
  (bind _asbp_paddle_r (Utilities|Casting|CastToBP_Paddle_R OtherActor)
    (:then
      (bind _returnvalue (Physics|GetPhysicsLinearVelocity (Variables|Default|GetStaticMesh) "None"))
      (Physics|SetPhysicsLinearVelocity (Variables|Default|GetStaticMesh) (Math|Vector|MakeVector (+ (.X (Math|Vector|BreakVector (Transformation|GetVelocity _asbp_paddle_r))) (Math|Random|RandomFloatinRange -1e+03 1e+03)) (* (.Y (Math|Vector|BreakVector _returnvalue)) -1.0) (.Z (Math|Vector|BreakVector _returnvalue))) false "None")
      (Audio|PlaySoundatLocation "/Game/Audio/S_ballCollision.S_ballCollision" "0, 0, 0"))
    (:CastFailed
      (bind _asbp_enemy_paddle (Utilities|Casting|CastToBP_Enemy_Paddle OtherActor)
        (:then
          (bind _returnvalue_2 (Physics|GetPhysicsLinearVelocity (Variables|Default|GetStaticMesh) "None"))
          (Physics|SetPhysicsLinearVelocity (Variables|Default|GetStaticMesh) (Math|Vector|MakeVector (+ (.X (Math|Vector|BreakVector (Transformation|GetVelocity _asbp_enemy_paddle))) (Math|Random|RandomFloatinRange -1e+03 1e+03)) (* (.Y (Math|Vector|BreakVector _returnvalue_2)) -1.0) (.Z (Math|Vector|BreakVector _returnvalue_2))) false "None")
          (Audio|PlaySoundatLocation "/Game/Audio/S_ballCollision.S_ballCollision" "0, 0, 0"))
        (:CastFailed
          (Utilities|Casting|CastToBP_HorizontalBoundary OtherActor
            (:then
              (bind _returnvalue_3 (Physics|GetPhysicsLinearVelocity (Variables|Default|GetStaticMesh) "None"))
              (Physics|SetPhysicsLinearVelocity (Variables|Default|GetStaticMesh) (Math|Vector|MakeVector (* (.X (Math|Vector|BreakVector _returnvalue_3)) -1.0) (.Y (Math|Vector|BreakVector _returnvalue_3)) (.Z (Math|Vector|BreakVector _returnvalue_3))) false "None")
              (Audio|PlaySoundatLocation "/Game/Audio/S_ballCollision.S_ballCollision" "0, 0, 0"))
            (:CastFailed
              (Utilities|Casting|CastToBP_L_Goal OtherActor
                (:then
                  (Transformation|SetActorLocation "0, 0, 0" false false)
                  (Physics|SetPhysicsLinearVelocity (Variables|Default|GetStaticMesh) "0,2000.000000, 0" false "None")
                  (Audio|PlaySoundatLocation "/Game/Audio/S_ballGoal.S_ballGoal" "0, 0, 0")
                  (Variables|Default|SetRPlayer_Score (+ (Variables|Default|GetRPlayer_Score) 1))
                  (bind _outactors (Actor|GetAllActorsOfClass "/Script/Engine.TextRenderActor"))
                  (for _array_element _outactors
                    (bind _astext_render_actor (Utilities|Casting|CastToTextRenderActor _array_element))
                    (if (Components|ComponentHasTag (Variables|/Script/Engine.TextRenderActor|GetTextRender _astext_render_actor) "Rplayer_Score_Tag")
                      (Rendering|Components|TextRender|SetText (Variables|/Script/Engine.TextRenderActor|GetTextRender _astext_render_actor) (Utilities|Text|ToText(Integer) (Variables|Default|GetRPlayer_Score)))
                      (if (> (Variables|Default|GetRPlayer_Score) 10)
                        (Development|PrintString "Right Side Wins!")
                        (Variables|Default|SetbGameOver true)))))
                (:CastFailed
                  (Utilities|Casting|CastToBP_R_Goal OtherActor)
                  (Transformation|SetActorLocation "0, 0, 0" false false)
                  (Physics|SetPhysicsLinearVelocity (Variables|Default|GetStaticMesh) "0,-2000.000000, 0" false "None")
                  (Audio|PlaySoundatLocation "/Game/Audio/S_ballGoal.S_ballGoal" "0, 0, 0")
                  (Variables|Default|SetLPlayer_Score (+ (Variables|Default|GetLPlayer_Score) 1))
                  (bind _outactors_2 (Actor|GetAllActorsOfClass "/Script/Engine.TextRenderActor"))
                  (for _array_element_2 _outactors_2
                    (bind _astext_render_actor_2 (Utilities|Casting|CastToTextRenderActor _array_element_2))
                    (if (Components|ComponentHasTag (Variables|/Script/Engine.TextRenderActor|GetTextRender _astext_render_actor_2) "LPlayer_Score_Tag")
                      (Rendering|Components|TextRender|SetText (Variables|/Script/Engine.TextRenderActor|GetTextRender _astext_render_actor_2) (Utilities|Text|ToText(Integer) (Variables|Default|GetLPlayer_Score)))
                      (if (> (Variables|Default|GetLPlayer_Score) 10)
                        (Development|PrintString "Left Side Wins!")
                        (Variables|Default|SetbGameOver true)))))))))))))

(event EventTick
  (params (DeltaSeconds :type Float%20%28single-precision%29))
  (if (Variables|Default|GetbGameOver)
    (Physics|SetPhysicsLinearVelocity (Variables|Default|GetStaticMesh) "0, 0, 0" false "None")
    (Utilities|FlowControl|Delay 3.0)
    (Game|OpenLevel(byName) "P1_Main")))

(fn ConstructionScript)